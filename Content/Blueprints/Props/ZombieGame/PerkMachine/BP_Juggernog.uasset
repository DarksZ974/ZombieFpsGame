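; Juggernog perk machine for the zombie game, which grants its indexed perk to the first-person player on interact.
; A power event plays a timeline that ramps material glow and toggles the spotlight, enabling interaction once the forward play finishes.
; Powering off disables interaction immediately and reverses the effect; BeginPlay applies the initial power state.
; Query functions report power state, interactability, prompt text and price, with no cost deducted here.
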(event `self.ReceiveBeginPlay`
  (`self.Power` (`self.Power On`)))

(event `Power`
  (params (On :type Boolean))
  (if On
    (bind (_direction _newtrack_0) (`Timeline|Timeline` :!via `PlayFromStart` :!label _label)
      (:`Update`
        (bind _output_get (set `self.PowerA` _newtrack_0))
        (`SceneComponent.SetVisibility` (`self.SpotLight`) (select `bool` (> _output_get 0.6) :`true` true) false)
        (`MeshComponent.SetScalarParameterValueOnMaterials` (`self.StaticMesh`) "Glow" (`KismetMathLibrary.Lerp` 0.0 0.01 (`self.PowerA`))))
      (:`Finished`
        (switch `ETimelineDirection` _direction
          (:`Forward`
            (set `self.Interactable ` true)
            (set `self.Power On` true)))))
    (else
      (set `self.Interactable ` false)
      (set `self.Power On` false)
      (goto _label :!via `Reverse`))))

(event `/Game/Blueprints/BPI_Interact.OnInteract`
  (params (Ammo :type Boolean) (AmmoSlot :type Integer))
  (bind _asbp_first_person_character (cast `/Game/FirstPerson/Blueprints/BP_FirstPersonCharacter` (`GameplayStatics.GetPlayerCharacter` 0)))
  (`/Game/FirstPerson/Blueprints/BP_FirstPersonCharacter.AddPerk` _asbp_first_person_character (`self.Index`)))

(fn `Interactable`
  (returns (Interactable :type Boolean) (Power :type Boolean) (PowerOn :type Boolean))
  (return (`self.Interactable `) true (`self.Power On`)))

(fn `Is Interactble / Get`
  (returns (Type :type "/Game/Blueprints/Enum/InteractSelection Enum") (Text :type Text) (Price :type Integer) (InteractableIndex :type Integer))
  (return "NewEnumerator5" "Buy Juggernog" (`self.Price`) (`self.Index`)))

(fn `UserConstructionScript`)