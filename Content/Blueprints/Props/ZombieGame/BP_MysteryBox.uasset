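; Zombie-mode mystery box that, once bought, offers the player a random weapon to take before the box closes.
; Timelines animate lid and weapon while a recursive, slowing Spin cycles DT_Weapon meshes, skipping both held weapons and the previous pick.
; Teddy odds rise with spin count; a teddy plays the departure sequence, hides the box and calls SetMysteryLocation on the game mode.
; A sky laser material fades with box activation and departure.
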(event `self.ReceiveTick`
  (params (DeltaSeconds :type "Float (single-precision)"))
  (`self.SkyLazerOpacity`))

(event `self.ReceiveBeginPlay`
  (`TimelineComponent.SetPlayRate` (`self.Timeline`) (/ 1.0 (`self.OpenTime`)))
  (`TimelineComponent.SetPlayRate` (`self.Timeline_0`) (/ 1.0 (`self.CloseTime`))))

(event `/Game/Blueprints/BPI_Interact.OnInteract`
  (params (Ammo :type Boolean) (AmmoSlot :type Integer))
  ;[1 1 1] Set interaction
  (if (`self.Can_Interact`)
    (switch `/Game/Blueprints/Enum/InteractSelection` (`self.Interact Type`)
      (:`NewEnumerator1`
        (set `self.Can_Interact` false)
        (set `self.Interact Type` "NewEnumerator4")
        (`SceneComponent.SetVisibility` (`self.Weapon`) false false)
        (bind _asbp_first_person_character (cast `/Game/FirstPerson/Blueprints/BP_FirstPersonCharacter` (`GameplayStatics.GetPlayerCharacter` 0)))
        (`/Game/FirstPerson/Blueprints/BP_FirstPersonCharacter.SetNewWeaponSlot` _asbp_first_person_character (`self.Spin_Last_Index`))
        (`self.Close`))
      (:`NewEnumerator3`
        (set `self.Can_Interact` false)
        (set `self.Interact Type` "NewEnumerator4")
        (`SceneComponent.SetVisibility` (`self.Weapon`) true false)
        (bind _asbp_first_person_character_2 (cast `/Game/FirstPerson/Blueprints/BP_FirstPersonCharacter` (`GameplayStatics.GetPlayerCharacter` 0)))
        (bind _weaponslots (`/Game/FirstPerson/Blueprints/BP_FirstPersonCharacter.WeaponSlots` _asbp_first_person_character_2))
        (bind _output_weaponindex (break `/Game/Blueprints/Structures/Weapon_Slot` (`|GetArrayItem` _weaponslots 1)))
        (set `self.S1WeaponIndex` _output_weaponindex)
        (bind _output_weaponindex_2 (break `/Game/Blueprints/Structures/Weapon_Slot` (`|GetArrayItem` _weaponslots 2)))
        (set `self.S2WeaponIndex` _output_weaponindex_2)
        (bind _outrownames (`DataTableFunctionLibrary.GetDataTableRowNames` "/Game/Blueprints/DataTables/DT_Weapon.DT_Weapon"))
        (for _array_element _outrownames
          (`|GetDataTableRow` "/Game/Blueprints/DataTables/DT_Weapon.DT_Weapon" _array_element
            (:`then`
              (`/Engine/EditorBlueprintResources/StandardMacros.IncrementInt` (`self.RowAmmount`)))))
        (`self.Open`)))))

(event `Open`
  ;[1 1 1] Open and close box
  (`GameplayStatics.PlaySound2D` "/Game/UI/SFX/BoxSounds/openBox.openBox" 1.0 1.0 0.0 null null)
  (`self.Spin`)
  (`GameplayStatics.PlaySound2D` "/Game/UI/SFX/BoxSounds/BoxMusic.BoxMusic" 1.0 1.0 0.0 null null)
  (bind (_direction _newtrack_0) (`Timeline|Timeline` :!via `PlayFromStart` :!label _label)
    (:`Update`
      (`SceneComponent.K2_SetRelativeRotation` (`self.Top_Scene`) (`KismetMathLibrary.RLerp` (struct) (struct :`Roll` -80.0) _newtrack_0) false false)
      (`SceneComponent.K2_SetRelativeLocation` (`self.Weapon`) (`KismetMathLibrary.VLerp` (`KismetMathLibrary.MakeVector` (`self.LocationX`)) (select `ETimelineDirection` _direction :`Forward` (`KismetMathLibrary.MakeVector` (`self.LocationX`) 0.0 90.0) :`Backward` (`self.WeaponLocation`)) _newtrack_0) false false))
    (:`Finished`
      (switch `ETimelineDirection` _direction
        (:`Backward`
          (if (`self.teddy`)
            (set `self.teddy` false)
            (else
              (set `self.Interact Type` "NewEnumerator3")
              (set `self.Can_Interact` true)))
          (set `self.Spin_Last_Index` 0)
          (set `self.RowAmmount` 0)
          (set `self.SpinIndex` 1)
          (`SceneComponent.SetVisibility` (`self.Weapon`) false false))))))

(event `Close`
  (bind (_relativelocation_x _relativelocation_y _relativelocation_z) (`KismetMathLibrary.BreakVector` (`SceneComponent.RelativeLocation` (`self.Weapon`))))
  ;[1 1 1] Open and close box
  (if (not (`self.teddy`))
    (`GameplayStatics.PlaySound2D` "/Game/UI/SFX/BoxSounds/closeBox.closeBox" 1.0 1.0 0.0 null null))
  (set `self.WeaponLocation` (`KismetMathLibrary.MakeVector` (`self.LocationX`) _relativelocation_y _relativelocation_z))
  (goto _label :!via `ReverseFromEnd`))

(event `Spin`
  (bind _spinweaponindex (`self.SpinWeaponIndex`))
  ;[1 1 1] Spin box function
  (if (<= (`self.SpinIndex`) 50)
    (set `self.SpinWeaponIndex` (`KismetMathLibrary.RandomIntegerInRange` 1 (`self.RowAmmount`)))
    (if (and (!= _spinweaponindex (`self.S1WeaponIndex`)) (!= _spinweaponindex (`self.S2WeaponIndex`)) (!= _spinweaponindex (`self.Spin_Last_Index`)))
      (`KismetSystemLibrary.Delay` (/ (`KismetMathLibrary.FClamp` (- (`KismetMathLibrary.Conv_IntToDouble` (`self.SpinIndex`)) 25.0) 1.0 50.0) 100.0))
      (if (== (`self.SpinIndex`) 49)
        (`self.TeddyFunc`)
        (if (`self.teddy`)
          (`SceneComponent.SetVisibility` (`self.Weapon`) false false)
          (`SceneComponent.SetVisibility` (`self.tedy`) true false)
          (`GameplayStatics.PlaySound2D` "/Game/UI/SFX/BoxSounds/boxLaughtTeddy.boxLaughtTeddy" 1.0 1.0 0.0 null null)
          (`KismetSystemLibrary.Delay` 1.0)
          (`self.TeddyAnim`)
          (else
            (`/Engine/EditorBlueprintResources/StandardMacros.IncrementInt` (`self.NbOfSpin`)
              (:`  `
                (bind _returnvalue (`|GetDataTableRow` "/Game/Blueprints/DataTables/DT_Weapon.DT_Weapon" (`KismetStringLibrary.Conv_StringToName` (`KismetStringLibrary.Conv_IntToString` (`self.SpinWeaponIndex`))) :!label _label_2)
                  (:`then`
                    (`SkeletalMeshComponent.SetSkeletalMeshAsset` (`self.Weapon`) (break `/Game/Blueprints/Structures/Weapon_Stat` _returnvalue))
                    (set `self.Spin_Last_Index` (`self.SpinWeaponIndex`))
                    (`/Engine/EditorBlueprintResources/StandardMacros.IncrementInt` (`self.SpinIndex`)
                      (:`  `
                        (`self.Spin`)))))))))
        (else
          (goto _label_2)))
      (else
        (`self.Spin`)))
    (else
      (set `self.Interact Type` "NewEnumerator1")
      (set `self.Can_Interact` true)
      (`self.CloseLoop`))))

(event `CloseLoop`
  (bind _locationx (`self.LocationX`))
  ;[1 1 1] Close loop function
  (bind (_direction _newtrack_0) (`Timeline|Timeline_0` :!via `PlayFromStart`)
    (:`Update`
      (`SceneComponent.K2_SetRelativeLocation` (`self.Weapon`) (`KismetMathLibrary.VLerp` (`KismetMathLibrary.MakeVector` _locationx 0.0 90.0) (`KismetMathLibrary.MakeVector` _locationx 0.0 60.0) _newtrack_0) false false))
    (:`Finished`
      (if (`|EnumEquality` (`self.Interact Type`) "NewEnumerator1")
        (set `self.Can_Interact` false)
        (set `self.Interact Type` "NewEnumerator4")
        (`self.Close`)))))

(event `SetMysteryBox`
  (params (SpawnFirst :type Boolean))
  ;[1 1 1] Set the mystery box
  (set `self.Spawn First` SpawnFirst)
  (`KismetSystemLibrary.Delay` 0.2)
  (bind (_direction _newtrack_0) (`Timeline|Timeline_1` :!via `PlayFromStart`)
    (:`Update`
      (`MeshComponent.SetScalarParameterValueOnMaterials` (`self.LazerLight`) "Fade" (`KismetMathLibrary.Lerp` 0.0 1.0 _newtrack_0))
      (if (>= (`TimelineComponent.GetPlaybackPosition` (`self.Timeline_1`)) 3.0)
        (`MeshComponent.SetScalarParameterValueOnMaterials` (`self.LazerLight`) "Fade" (`KismetMathLibrary.Lerp` 0.0 (`self.LightFadeCalcul`) _newtrack_0))))
    (:`Finished`
      (set `self.NbOfSpin` 0)
      (`self.SetBoxEnable` true)
      (set `self.MysteryBoxUse` true))))

(event `TeddyAnim`
  (bind _tedy (`self.tedy`))
  ;[1 1 1] Teddy Animation
  (`KismetSystemLibrary.Delay` 1.5)
  (bind (_direction _newtrack_0) (`Timeline|Timeline_2` :!via `PlayFromStart`)
    (:`Update`
      (`SceneComponent.K2_SetRelativeLocation` (`self.tedy`) (`KismetMathLibrary.MakeVector` 0.0 0.0 _newtrack_0) false false))
    (:`Finished`
      (`GameplayStatics.PlaySound2D` "/Game/UI/SFX/BoxSounds/boxDisappear.boxDisappear" 1.0 1.0 0.0 null null)
      (`SceneComponent.SetVisibility` _tedy false false)
      (`SceneComponent.K2_SetRelativeLocation` _tedy (0.0 0.0 80.0) false false)
      (`self.BoxAnim`)
      (`KismetSystemLibrary.Delay` 2.0)
      (`self.Close`)
      (`GameplayStatics.PlaySound2D` "/Game/UI/SFX/BoxSounds/boxWoosh.boxWoosh" 1.0 1.0 0.0 null null)
      (`GameplayStatics.PlaySound2D` "/Game/UI/SFX/BoxSounds/boxSpinDisparition.boxSpinDisparition" 1.0 1.0 0.0 null null)
      (`KismetSystemLibrary.Delay` 5.0)
      (`GameplayStatics.PlaySound2D` "/Game/UI/SFX/BoxSounds/boxPoof.boxPoof" 1.0 1.0 0.0 null null)
      (`self.SetBoxEnable` false)
      (`KismetSystemLibrary.Delay` 5.0)
      (bind _asbp_zombie_game_mode (cast `/Game/Blueprints/BP_ZombieGameMode` (`GameplayStatics.GetGameMode`)))
      (`/Game/Blueprints/BP_ZombieGameMode.SetMysteryLocation` _asbp_zombie_game_mode false)
      (bind (_direction_2 _newtrack_0_2) (`Timeline|Timeline_3` :!via `PlayFromStart`)
        (:`Update`
          (`MeshComponent.SetScalarParameterValueOnMaterials` (`self.LazerLight`) "Fade" (`KismetMathLibrary.Lerp` (`self.LightFadeCalcul`) 0.0 _newtrack_0_2)))
        (:`Finished`
          (set `self.MysteryBoxUse` false))))))

(event `SetBoxEnable`
  (params (Enable :type Boolean))
  ;[1 1 1] Enable the mystery box
  (if Enable
    (`self.SetActorHiddenInGame` self false)
    (set `self.Can_Interact` true)
    (set `self.Interact Type` "NewEnumerator3")
    (else
      (`self.SetActorHiddenInGame` self true))))

(event `BoxAnim`
  (bind _bottom (`self.Bottom`))
  (bind (_direction _newtrack_0) (`Timeline|Timeline_4` :!via `PlayFromStart`)
    (:`Update`
      (`SceneComponent.K2_SetRelativeLocation` _bottom (`KismetMathLibrary.MakeVector` 0.0 0.0 _newtrack_0) false false)
      (`KismetSystemLibrary.Delay` 1.5)
      (bind (_direction_2 _newtrack_0_2) (`Timeline|Timeline_5` :!via `PlayFromStart`)
        (:`Update`
          (`SceneComponent.K2_SetRelativeRotation` _bottom (`KismetMathLibrary.RLerp` (struct) (struct :`Roll` 180.0) _newtrack_0_2) false false))))
    (:`Finished`
      (`SceneComponent.K2_SetRelativeLocation` (`self.Bottom`) (0.0 0.0 18.0) false false))))

(fn `Interactable`
  (returns (Interactable :type Boolean) (Power :type Boolean) (PowerOn :type Boolean))
  (return (`self.Can_Interact`) false false))

(fn `Is Interactble / Get`
  (returns (Type :type "/Game/Blueprints/Enum/InteractSelection Enum") (Text :type Text) (Price :type Integer) (InteractableIndex :type Integer))
  (return (`self.Interact Type`) (select `/Game/Blueprints/Enum/InteractSelection` (`self.Interact Type`) :`NewEnumerator1` "take" :`NewEnumerator3` "open Mystery Box" :!type "Text") (`self.Price`) (`self.Spin_Last_Index`)))

(fn `SkyLazerOpacity`
  (if (`self.MysteryBoxUse`)
    (if (`PrimitiveComponent.IsOverlappingActor` (`self.SkyLazerLightCol`) (`GameplayStatics.GetPlayerCharacter` 0))
      (`MeshComponent.SetScalarParameterValueOnMaterials` (`self.LazerLight`) "Fade" (`self.LightFadeCalcul`)))))

(fn `TeddyFunc`
  (if (< (`self.NbOfSpin`) 4)
    (set `self.teddy` false)
    (elif (< (`self.NbOfSpin`) 8)
      (if (and (== (`self.NbOfSpin`) 7) (`self.FirstBox`))
        (set `self.teddy` true)
        (elif (<= (`KismetMathLibrary.RandomFloatInRange` 0.0 1.0) 0.15)
          (set `self.teddy` true)
          (else
            (set `self.teddy` false))))
      (elif (< (`self.NbOfSpin`) 12)
        (if (<= (`KismetMathLibrary.RandomFloatInRange` 0.0 1.0) 0.3)
          (set `self.teddy` true)
          (else
            (set `self.teddy` false)))
        (elif (<= (`KismetMathLibrary.RandomFloatInRange` 0.0 1.0) 0.5)
          (set `self.teddy` true)
          (else
            (set `self.teddy` false)))))))

(fn `UserConstructionScript`
  (`MeshComponent.SetScalarParameterValueOnMaterials` (`self.LazerLight`) "Fade" 0.0))