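; BP_Door is an interactable door for the zombie game that opens rooms, exposing a prompt text, price and power setting through interface functions.
; On interact, it compares the player's distance to two side markers and flags the far side's room in the game mode's SpawnOnOpenRoom array.
; It then disables interaction, moves the door along Z with a rate-scaled timeline, and destroys itself after the opening delay.
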(event `/Game/Blueprints/BPI_Interact.OnInteract`
  (params (Ammo :type Boolean) (AmmoSlot :type Integer))
  (bind _returnvalue (`SceneComponent.K2_GetComponentLocation` (`Character.CapsuleComponent` (`GameplayStatics.GetPlayerCharacter` 0))))
  (if (< (`KismetMathLibrary.Vector_Distance` _returnvalue (`SceneComponent.K2_GetComponentLocation` (`self.FirstSide`))) (`KismetMathLibrary.Vector_Distance` _returnvalue (`SceneComponent.K2_GetComponentLocation` (`self.SecondSide`))))
    (bind _asbp_zombie_game_mode (cast `/Game/Blueprints/BP_ZombieGameMode` (`GameplayStatics.GetGameMode`)))
    (`KismetArrayLibrary.Array_Set` (`/Game/Blueprints/BP_ZombieGameMode.SpawnOnOpenRoom` _asbp_zombie_game_mode) (`self.RoomNumber_2`) true true)
    (else
      (bind _asbp_zombie_game_mode_2 (cast `/Game/Blueprints/BP_ZombieGameMode` (`GameplayStatics.GetGameMode`)))
      (`KismetArrayLibrary.Array_Set` (`/Game/Blueprints/BP_ZombieGameMode.SpawnOnOpenRoom` _asbp_zombie_game_mode_2) (`self.RoomNumber`) true true)))
  (set `self.Interactable ` false)
  (`self.OpenDoor`))

(event `OpenDoor`
  (bind (_relativelocation_x _relativelocation_y _relativelocation_z) (`KismetMathLibrary.BreakVector` (`SceneComponent.RelativeLocation` (`self.Door`))))
  (`TimelineComponent.SetPlayRate` (`self.Timeline`) (/ 1.0 (`self.TimeOpening`)))
  (set `self.Start` (`SceneComponent.RelativeLocation` (`self.Door`)))
  (set `self.End` (`KismetMathLibrary.MakeVector` _relativelocation_x _relativelocation_y (+ _relativelocation_z (`self.ZValue`))))
  (bind (_direction _newtrack_0) (`Timeline|Timeline` :!via `PlayFromStart`)
    (:`Update`
      (`SceneComponent.K2_SetRelativeLocation` (`self.Door`) (`KismetMathLibrary.VLerp` (`self.Start`) (`self.End`) _newtrack_0) false false)
      (`KismetSystemLibrary.Delay` (`self.TimeOpening`))
      (`self.K2_DestroyActor`))))

(fn `Interactable`
  (returns (Interactable :type Boolean) (Power :type Boolean) (PowerOn :type Boolean))
  (return (`self.Interactable `) (`self.Power`) false))

(fn `Is Interactble / Get`
  (returns (Type :type "/Game/Blueprints/Enum/InteractSelection Enum") (Text :type Text) (Price :type Integer) (InteractableIndex :type Integer))
  (return "NewEnumerator3" (`self.Text`) (`self.Price`) 0))

(fn `UserConstructionScript`)