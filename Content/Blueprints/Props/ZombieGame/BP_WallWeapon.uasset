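; BP_WallWeapon is a wall-mounted weapon purchase prop for the zombie game, exposing its price and weapon index through interaction functions.
; On BeginPlay, a zero-length sphere trace snaps the weapon and sphere to the nearby surface, orienting the weapon to its normal.
; The weapon mesh comes from DT_Weapon by index.
; OnInteract either gives the first-person character that weapon or calls SetMaxAmmo on the supplied slot.
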(event `self.ReceiveBeginPlay`
  (bind _returnvalue (`SceneComponent.K2_GetComponentLocation` (`self.DefaultSceneRoot`)))
  (bind _outhit (`KismetSystemLibrary.SphereTraceSingle` _returnvalue _returnvalue 50.0 "TraceTypeQuery1"))
  (`SceneComponent.K2_SetWorldTransform` (`self.Weapon`) (`KismetMathLibrary.MakeTransform` (`.Location` (`GameplayStatics.BreakHitResult` _outhit)) (`KismetMathLibrary.Conv_VectorToRotator` (`.Normal` (`GameplayStatics.BreakHitResult` _outhit)))) false false)
  (`SceneComponent.K2_SetWorldLocation` (`self.Sphere`) (`.Location` (`GameplayStatics.BreakHitResult` _outhit)) false false)
  (bind _returnvalue_2 (`|GetDataTableRow` "/Game/Blueprints/Player/DT_Weapon.DT_Weapon" (`KismetStringLibrary.Conv_StringToName` (`KismetStringLibrary.Conv_IntToString` (`self.WeaponIndex`))))
    (:`then`
      (set `SkeletalMeshComponent.SkeletalMeshAsset` (break `/Game/Blueprints/Player/Weapon_Stat` _returnvalue_2) (`self.Weapon`)))))

(event `/Game/Blueprints/BPI_Interact.OnInteract`
  (params (Ammo :type Boolean) (AmmoSlot :type Integer))
  (if (not Ammo)
    (bind _asbp_first_person_character (cast `/Game/FirstPerson/Blueprints/BP_FirstPersonCharacter` (`GameplayStatics.GetPlayerCharacter` 0)))
    (`/Game/FirstPerson/Blueprints/BP_FirstPersonCharacter.SetNewWeaponSlot` _asbp_first_person_character (`self.WeaponIndex`))
    (else
      (bind _asbp_first_person_character_2 (cast `/Game/FirstPerson/Blueprints/BP_FirstPersonCharacter` (`GameplayStatics.GetPlayerCharacter` 0)))
      (`/Game/FirstPerson/Blueprints/BP_FirstPersonCharacter.SetMaxAmmo` _asbp_first_person_character_2 AmmoSlot))))

(fn `Interactable`
  (returns (Interactable :type Boolean) (Power :type Boolean) (PowerOn :type Boolean))
  (return false false false))

(fn `Is Interactble / Get`
  (returns (Type :type "/Game/Blueprints/Enum/InteractSelection Enum") (Text :type Text) (Price :type Integer) (InteractableIndex :type Integer))
  (locals (NewLocalVar :type Integer :default 500))
  (return "NewEnumerator2" "" (`self.Price`) (`self.WeaponIndex`)))

(fn `UserConstructionScript`)