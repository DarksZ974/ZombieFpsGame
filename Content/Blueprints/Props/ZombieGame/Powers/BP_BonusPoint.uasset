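; BP_BonusPoint is a bonus points power-up pickup for the zombie game mode.
; When BP_FirstPersonCharacter overlaps its sphere, it adds points and shows power-up text through the HUD widget, plays pickup and announcer sounds, then destroys itself.
; If left uncollected, it despawns on a timer, warning first with looping skeletal mesh visibility toggles, with a second, fast-flash loop starting alongside the first before removal.
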(event `self.ReceiveBeginPlay`
  (`KismetSystemLibrary.Delay` (`self.DelayDespawn`))
  (`self.Flashing`)
  (`KismetSystemLibrary.Delay` 5.0)
  (`self.FlashingFast`)
  (`KismetSystemLibrary.Delay` 5.0)
  (`self.K2_DestroyActor`))

(event `Flashing`
  (`SceneComponent.SetVisibility` (`self.SkeletalMesh`) false false :!label _label)
  (`KismetSystemLibrary.Delay` (`self.DelayRate`))
  (`SceneComponent.SetVisibility` (`self.SkeletalMesh`) true false)
  (`KismetSystemLibrary.Delay` (`self.DelayRate`))
  (goto _label))

(event `FlashingFast`
  (bind _skeletalmesh (`self.SkeletalMesh`))
  (`SceneComponent.SetVisibility` _skeletalmesh true false :!label _label_2)
  (`KismetSystemLibrary.Delay` (`self.DelayRate_0`))
  (`SceneComponent.SetVisibility` _skeletalmesh false false)
  (`KismetSystemLibrary.Delay` (`self.DelayRate_0`))
  (goto _label_2))

(event `self.Sphere.OnComponentBeginOverlap`
  (params (OverlappedComponent :type "PrimitiveComponent Object Reference") (OtherActor :type "Actor Object Reference") (OtherComp :type "PrimitiveComponent Object Reference") (OtherBodyIndex :type Integer) (bFromSweep :type Boolean) (SweepResult :type "HitResult Structure (by ref)"))
  (cast `/Game/FirstPerson/Blueprints/BP_FirstPersonCharacter` OtherActor)
  (bind _foundwidgets (`WidgetBlueprintLibrary.GetAllWidgetsOfClass` "/Game/UI/VFX/Screen/WGBlueprints/Hud.Hud_C"))
  (bind _output (`|GetArrayItem` _foundwidgets))
  (`/Game/UI/VFX/Screen/WGBlueprints/Hud.SetPowerUpText` _output "BONUS POINTS")
  (`/Game/UI/VFX/Screen/WGBlueprints/Hud.IncreasePoint` _output 1000)
  (`GameplayStatics.PlaySound2D` "/Game/UI/SFX/Power_up/PowerUpActive_End/PowerUp_Take.PowerUp_Take" 1.0 1.0 0.0 null null)
  (`KismetSystemLibrary.Delay` 0.5)
  (`GameplayStatics.PlaySound2D` "/Game/UI/SFX/Power_up/BonusPoint/Announcer_Bonus_Points_Zombies.Announcer_Bonus_Points_Zombies" 1.0 1.0 0.0 null null)
  (`self.K2_DestroyActor`))

(fn `UserConstructionScript`)