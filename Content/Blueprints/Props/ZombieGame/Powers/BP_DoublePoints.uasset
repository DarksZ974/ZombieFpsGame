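; BP_DoublePoints is the Double Points power-up pickup for the zombie game.
; On overlapping its sphere, the first-person character receives power-up 1, the HUD shows the power-up name, two sounds play and the actor destroys itself.
; An uncollected pickup waits out a despawn delay, then blinks its Double component through looping Delay visibility toggles, adding a second, differently timed blink loop before it despawns.
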(event `self.ReceiveBeginPlay`
  (`KismetSystemLibrary.Delay` (`self.DelayDespawn`))
  (`self.Flashing`)
  (`KismetSystemLibrary.Delay` 5.0)
  (`self.FlashingFast`)
  (`KismetSystemLibrary.Delay` 5.0)
  (`self.K2_DestroyActor`))

(event `Flashing`
  (`SceneComponent.SetVisibility` (`self.Double`) false false :!label _label)
  (`KismetSystemLibrary.Delay` (`self.DelayRate`))
  (`SceneComponent.SetVisibility` (`self.Double`) true false)
  (`KismetSystemLibrary.Delay` (`self.DelayRate`))
  (goto _label))

(event `FlashingFast`
  (bind _double (`self.Double`))
  (`SceneComponent.SetVisibility` _double true false :!label _label_2)
  (`KismetSystemLibrary.Delay` (`self.DelayRate_0`))
  (`SceneComponent.SetVisibility` _double false false)
  (`KismetSystemLibrary.Delay` (`self.DelayRate_0`))
  (goto _label_2))

(event `self.Sphere.OnComponentBeginOverlap`
  (params (OverlappedComponent :type "PrimitiveComponent Object Reference") (OtherActor :type "Actor Object Reference") (OtherComp :type "PrimitiveComponent Object Reference") (OtherBodyIndex :type Integer) (bFromSweep :type Boolean) (SweepResult :type "HitResult Structure (by ref)"))
  (bind _asbp_first_person_character (cast `/Game/FirstPerson/Blueprints/BP_FirstPersonCharacter` OtherActor))
  (`/Game/FirstPerson/Blueprints/BP_FirstPersonCharacter.AddPowerUp` _asbp_first_person_character 1)
  (bind _foundwidgets (`WidgetBlueprintLibrary.GetAllWidgetsOfClass` "/Game/UI/VFX/Screen/WGBlueprints/Hud.Hud_C"))
  (`/Game/UI/VFX/Screen/WGBlueprints/Hud.SetPowerUpText` (`|GetArrayItem` _foundwidgets) "DOUBLE POINTS")
  (`GameplayStatics.PlaySound2D` "/Game/UI/SFX/Power_up/PowerUpActive_End/PowerUp_Take.PowerUp_Take" 1.0 1.0 0.0 null null)
  (`GameplayStatics.PlaySound2D` "/Game/UI/SFX/Power_up/DoublePoints/COD_Black_Ops-Zombies-_Double_Points_Sound.COD_Black_Ops-Zombies-_Double_Points_Sound" 1.0 1.0 0.0 null null)
  (`self.K2_DestroyActor`))

(fn `UserConstructionScript`)