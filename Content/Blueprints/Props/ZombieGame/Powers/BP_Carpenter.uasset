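; BP_Carpenter is a Carpenter power-up pickup for the zombie game.
; After a configurable delay its Hammer mesh blinks, then a second, separately timed blink loop joins the first before the actor destroys itself.
; When BP_FirstPersonCharacter overlaps the Sphere, it sets the Hud power-up text, plays pickup, announcement and loop sounds, and destroys itself.
; The graph contains no repair effect.
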(event `self.ReceiveBeginPlay`
  (`KismetSystemLibrary.Delay` (`self.DelayDespawn`))
  (`self.Flashing`)
  (`KismetSystemLibrary.Delay` 5.0)
  (`self.FlashingFast`)
  (`KismetSystemLibrary.Delay` 5.0)
  (`self.K2_DestroyActor`))

(event `Flashing`
  (`SceneComponent.SetVisibility` (`self.Hammer`) false false :!label _label)
  (`KismetSystemLibrary.Delay` (`self.DelayRate`))
  (`SceneComponent.SetVisibility` (`self.Hammer`) true false)
  (`KismetSystemLibrary.Delay` (`self.DelayRate`))
  (goto _label))

(event `FlashingFast`
  (bind _hammer (`self.Hammer`))
  (`SceneComponent.SetVisibility` _hammer true false :!label _label_2)
  (`KismetSystemLibrary.Delay` (`self.DelayRate_0`))
  (`SceneComponent.SetVisibility` _hammer false false)
  (`KismetSystemLibrary.Delay` (`self.DelayRate_0`))
  (goto _label_2))

(event `self.Sphere.OnComponentBeginOverlap`
  (params (OverlappedComponent :type "PrimitiveComponent Object Reference") (OtherActor :type "Actor Object Reference") (OtherComp :type "PrimitiveComponent Object Reference") (OtherBodyIndex :type Integer) (bFromSweep :type Boolean) (SweepResult :type "HitResult Structure (by ref)"))
  (cast `/Game/FirstPerson/Blueprints/BP_FirstPersonCharacter` OtherActor)
  (bind _foundwidgets (`WidgetBlueprintLibrary.GetAllWidgetsOfClass` "/Game/UI/VFX/Screen/WGBlueprints/Hud.Hud_C"))
  (`/Game/UI/VFX/Screen/WGBlueprints/Hud.SetPowerUpText` (`|GetArrayItem` _foundwidgets) "CARPENTER")
  (`GameplayStatics.PlaySound2D` "/Game/UI/SFX/Power_up/PowerUpActive_End/PowerUp_Take.PowerUp_Take" 1.0 1.0 0.0 null null)
  (`GameplayStatics.PlaySound2D` "/Game/UI/SFX/Power_up/Carpenter/cod_zombiescarpenter_power_up_sound.cod_zombiescarpenter_power_up_sound" 1.0 1.0 0.0 null null)
  (`GameplayStatics.SpawnSound2D` "/Game/UI/SFX/Power_up/Carpenter/Carpenter_Full_Loop.Carpenter_Full_Loop" 1.0 1.0 0.0 null)
  (`self.K2_DestroyActor`))

(fn `UserConstructionScript`)