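; BP_PlayerF1 is a player Blueprint with a cursor-driven look camera and an unfinished weapon system.
; BeginPlay shows the cursor in Game and UI input mode.
; Tick restarts a Timeline that lerps the camera toward the deprojected mouse position, clamping pitch and yaw.
; FireWeapon's single-shot case only draws a Visibility line trace along camera velocity, not forward vector; SetWeaponStats and EquipWeapon are empty.
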(event `self.ReceiveBeginPlay`
  (bind _returnvalue (`GameplayStatics.GetPlayerController` 0))
  (`WidgetBlueprintLibrary.SetInputMode_GameAndUIEx` _returnvalue null "DoNotLock" false)
  (set `PlayerController.bShowMouseCursor` true _returnvalue))

(event `self.ReceiveTick`
  (params (DeltaSeconds :type "Float (single-precision)"))
  (bind _camera (`self.Camera`))
  (bind (_direction _newtrack_0) (`Timeline|Timeline` :!via `PlayFromStart`)
    (:`Update`
      (bind (_returnvalue_roll _returnvalue_pitch _returnvalue_yaw) (`KismetMathLibrary.BreakRotator` (`KismetMathLibrary.RLerp` (`SceneComponent.K2_GetComponentRotation` _camera) (`KismetMathLibrary.FindLookAtRotation` (`SceneComponent.K2_GetComponentLocation` _camera) (`PlayerController.DeprojectMousePositionToWorld` (`GameplayStatics.GetPlayerController` 0))) _newtrack_0)))
      (`SceneComponent.K2_SetWorldRotation` _camera (`KismetMathLibrary.MakeRotator` _returnvalue_roll (`KismetMathLibrary.FClamp` _returnvalue_pitch -60.0 10.0) (`KismetMathLibrary.FClamp` _returnvalue_yaw -65.0 12.0)) false false))))

(fn `EquipWeapon`)

(fn `FireWeapon`
  (bind _camera (`self.Camera`))
  (bind _returnvalue (`SceneComponent.K2_GetComponentLocation` _camera))
  (switch `/Game/Blueprints/Enum/FireType` (`self.Weapon Info Fire Type`)
    (:`NewEnumerator0`
      (`KismetSystemLibrary.LineTraceSingle` :`Start` _returnvalue :`End` (+ _returnvalue (* (`SceneComponent.GetComponentVelocity` _camera) 25000.0)) :`TraceChannel` "TraceTypeQuery1" :`DrawDebugType` "ForDuration"))))

(fn `SetWeaponStats`
  (locals (WeaponInfo :type "/Game/Blueprints/Structures/Weapon_Stat Structure")))

(fn `UserConstructionScript`)