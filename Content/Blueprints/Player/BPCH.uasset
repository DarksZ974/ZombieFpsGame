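; BPCH is a player health Blueprint that handles damage and healing through two functions.
; RemoveHealt and AddHealt adjust current health, clamped between zero and the maximum.
; Unless NotEnemyHit is set, RemoveHealt calls OnHit on the first top-level Hud widget with the enemy reference, then returns whether health is depleted.
; The event graph has no active logic.
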(fn `AddHealt`
  (params (Ammount :type "Float (double-precision)"))
  (set `self.HealtCurrent` (`KismetMathLibrary.FClamp` (+ (`self.HealtCurrent`) Ammount) 0.0 (`self.HealtMax`))))

(fn `RemoveHealt`
  (params (Ammount :type "Float (double-precision)") (EnemyRef :type "Actor Object Reference") (NotEnemyHit :type Boolean))
  (returns (Dead :type Boolean))
  (bind _output_get (set `self.HealtCurrent` (`KismetMathLibrary.FClamp` (- (`self.HealtCurrent`) Ammount) 0.0 (`self.HealtMax`))))
  (if (not NotEnemyHit)
    (bind _foundwidgets (`WidgetBlueprintLibrary.GetAllWidgetsOfClass` "/Game/UI/VFX/Screen/WGBlueprints/Hud.Hud_C"))
    (`/Game/UI/VFX/Screen/WGBlueprints/Hud.OnHit` (`|GetArrayItem` _foundwidgets) EnemyRef)
    (return (<= _output_get 0.0))))