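; Game mode for a round-based zombie game: BeginPlay disables player input and adds the start and HUD widgets, then LevelGameStart enables input and begins the first round.
; IncreaseRound advances the round and resets its power-up count, while Nuke pauses spawning for five seconds; CheckEndRound is empty.
; It numbers Mystery Boxes, then randomly reveals one other than the current, retrying until one is picked.
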(event `LevelGameStart`
  (`self.EnableInput` (`GameplayStatics.GetPlayerCharacter` 0) (`GameplayStatics.GetPlayerController` 0))
  (`self.Increase Round`)
  (`self.SetMysteryBox`)
  (`self.SetMysteryLocation` true))

(event `self.ReceiveBeginPlay`
  (bind _returnvalue (`GameplayStatics.GetPlayerController` 0))
  (`self.DisableInput` (`GameplayStatics.GetPlayerCharacter` 0) _returnvalue)
  (`WidgetBlueprintLibrary.SetInputMode_GameOnly` _returnvalue)
  (bind _returnvalue_2 (`|CreateWidget` "/Game/UI/VFX/Screen/WGBlueprints/StartLevel.StartLevel_C"))
  (`UserWidget.AddToViewport` _returnvalue_2 0)
  (bind _returnvalue_3 (`|CreateWidget` "/Game/UI/VFX/Screen/WGBlueprints/Hud.Hud_C" null self))
  (`UserWidget.AddToViewport` _returnvalue_3 0))

(event `Nuke`
  (set `self.Spawn` false)
  (bind _outactors (`GameplayStatics.GetAllActorsOfClass` null))
  (for _ _outactors
    _)
  (`KismetSystemLibrary.Delay` 5.0)
  (set `self.Spawn` true))

(event `CheckEndRound`)

(event `Increase Round`
  (set `self.PowerUpSpawn/Round` 0)
  (`/Engine/EditorBlueprintResources/StandardMacros.IncrementInt` (`self.RoundNumber`)))

(fn `SetMysteryBox`
  (set `self.NbMysteryBox` 0)
  (bind _outactors (`GameplayStatics.GetAllActorsOfClass` "/Game/Blueprints/Props/ZombieGame/BP_MysteryBox.BP_MysteryBox_C"))
  (for (_array_element _array_index) _outactors
    (set `/Game/Blueprints/Props/ZombieGame/BP_MysteryBox.MysteryBoxNum` (+ _array_index 1) _array_element)
    (`/Engine/EditorBlueprintResources/StandardMacros.IncrementInt` (`self.NbMysteryBox`))))

(fn `SetMysteryLocation`
  (params (Initial :type Boolean))
  (locals (FirstSpawn :type Boolean) (MysteryBoxTemp :type "Float (double-precision)" :default 0.0) (Set :type Boolean))
  (set `local.FirstSpawn` Initial)
  (set `local.MysteryBoxTemp` (`KismetMathLibrary.Conv_IntToDouble` (`self.NbMysteryBox`)))
  (bind _outactors (`GameplayStatics.GetAllActorsOfClass` "/Game/Blueprints/Props/ZombieGame/BP_MysteryBox.BP_MysteryBox_C"))
  (for _array_element _outactors :!label _label
    (if (not (`local.Set`))
      (if (and (<= (`KismetMathLibrary.RandomFloatInRange` 0.0 1.0) (/ 1.0 (`local.MysteryBoxTemp`))) (!= (`/Game/Blueprints/Props/ZombieGame/BP_MysteryBox.MysteryBoxNum` _array_element) (`self.CurrentMysteryBox`)))
        (set `self.CurrentMysteryBox` (`/Game/Blueprints/Props/ZombieGame/BP_MysteryBox.MysteryBoxNum` _array_element))
        (`self.SetActorHiddenInGame` _array_element false)
        (`/Game/Blueprints/Props/ZombieGame/BP_MysteryBox.SetMysteryBox` _array_element (`local.FirstSpawn`))
        (set `local.Set` true)
        (else
          (`/Engine/EditorBlueprintResources/StandardMacros.DecrementFloat` (`local.MysteryBoxTemp`))))))
  (if (not (`local.Set`))
    (goto _label)))

(fn `UserConstructionScript`)